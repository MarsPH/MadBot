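; BP_SmallSphere is a short-lived moving sphere actor that tumbles as it travels and winks out after its lifetime.
; On BeginPlay it picks a random scaled rotation rate and starts a timer for LifeTime.
; Each Tick moves the mesh along its own forward vector at MoveSpeed while rotating it, so its heading keeps changing.
; When the timer fires, a timeline drives the actor's scale, then destroys it on finish.
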(event `self.ReceiveBeginPlay`
  (`self.InitializaeDeltaRotation`)
  (`KismetSystemLibrary.K2_SetTimerDelegate` (delegate `WinkOut`) (`self.LifeTime`)))

(event `WinkOut`
  (bind (_direction _scale) (`Timeline|WinkoutTimeLine`)
    (:`Update`
      (`self.SetActorScale3D` (`KismetMathLibrary.MakeVector` _scale _scale _scale)))
    (:`Finished`
      (`self.K2_DestroyActor`))))

(event `self.ReceiveTick`
  (params (DeltaSeconds :type "Float (single-precision)"))
  (`self.UpdateLocation` DeltaSeconds)
  (`self.UpdateRotation`))

(fn `InitializaeDeltaRotation`
  (set `self.Delta Rotation` (* (`KismetMathLibrary.RandomRotator` false) (`self.DeltaRotationScale`))))

(fn `UpdateLocation`
  (params (DeltaSceonds :type "Float (single-precision)"))
  (`SceneComponent.K2_AddWorldOffset` (`self.ShpereMesh`) (* DeltaSceonds (`SceneComponent.GetForwardVector` (`self.ShpereMesh`)) (`self.MoveSpeed`)) false false))

(fn `UpdateRotation`
  (`SceneComponent.K2_AddWorldRotation` (`self.ShpereMesh`) (* (`self.Delta Rotation`) (`GameplayStatics.GetWorldDeltaSeconds`)) false false))

(fn `UserConstructionScript`)