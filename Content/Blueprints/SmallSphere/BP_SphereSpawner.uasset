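; BP_SphereSpawner is an actor that keeps spawning BP_SmallSphere actors around itself.
; On BeginPlay it starts a looping timer at SpawnTime intervals, and each firing spawns one sphere with a random rotation.
; SetRandomLocationWithinSphere picks each spawn point by offsetting the spawner's location along a random rotation's forward vector by a random distance up to SpawnRange.
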(event `self.ReceiveBeginPlay`
  ;[0.1615 0.02571 0.01285] Spawn Spheres
  (`KismetSystemLibrary.K2_SetTimerDelegate` (delegate `SpawnSpheres`) (`self.SpawnTime`) true))

(event `SpawnSpheres`
  ;[0.1615 0.02571 0.01285] Spawn Spheres
  (`|SpawnActorFromClass` "/Game/Blueprints/SmallSphere/BP_SmallSphere.BP_SmallSphere_C" (`KismetMathLibrary.MakeTransform` (`self.SetRandomLocationWithinSphere`) (`KismetMathLibrary.RandomRotator` false)) "Undefined" "MultiplyWithRoot" null null))

(event `self.ReceiveTick`
  (params (DeltaSeconds :type "Float (single-precision)")))

(fn `SetRandomLocationWithinSphere`
  (returns (ReturnValue :type "Vector Structure"))
  (return (+ (`self.K2_GetActorLocation`) (* (`KismetMathLibrary.GetForwardVector` (`KismetMathLibrary.RandomRotator` false)) (`KismetMathLibrary.RandomFloatInRange` 0.0 (`self.SpawnRange`))))))

(fn `UserConstructionScript`)